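; Gameplay ability for enemy melee attacks, turning the avatar to face its combat target and playing a random tagged attack montage.
; A gameplay event matching the montage's tag triggers a small sphere query at that tag's combat socket, damaging live players not on the avatar's team.
; The ability ends after that hit check or when the montage completes, is interrupted or is cancelled.
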(event Ability|EventActivateAbility
  (bind _returnvalue (Ability|GetAvatarActorfromActorInfo))
  (bind _returnvalue_2 (Ability|GetAvatarActorfromActorInfo))
  (bind _returnvalue_3 (Class|EnemyInterface|GetCombatTarget(Message) _returnvalue))
  (bind _ascombat_interface (Utilities|Casting|CastToCombatInterface _returnvalue))
  (Class|CombatInterface|UpdateFacingTarget _ascombat_interface (Transformation|GetActorLocation _returnvalue_3))
  (bind _returnvalue_4 (Class|CombatInterface|GetAttackMontages(Message) _returnvalue))
  (bind _output_get (Variables|Default|SetTaggedMontage (.OutItem (Utilities|Array|Random _returnvalue_4))))
  (|PlayMontageandWaitProxy "None" (.Montage (Utilities|Struct|BreakTagMontage _output_get)) 1.0 "None" false 1.0 0.0 false
    (:then
      (Ability|Tasks|WaitGameplayEvent (.MontageTag (Utilities|Struct|BreakTagMontage _output_get)) 0
        (:EventReceived
          (bind _returnvalue_5 (Class|CombatInterface|GetCombatSocketLocation(Message) _returnvalue_2 (.MontageTag (Utilities|Struct|BreakTagMontage _output_get))))
          (bind _outoverlappingactor (Class|AuraAbilitySystemLibrary|GetLivePlayersWithinRadius _returnvalue_2 (Utilities|Array|MakeArray _returnvalue_2) _returnvalue_5 45.0))
          (for _array_element _outoverlappingactor
            (if (not (Class|AuraAbilitySystemLibrary|IsonSameTeam _array_element (Ability|GetAvatarActorfromActorInfo)))
              (Class|AuraDamageGameplayAbility|CauseDamage _array_element)))
          (Ability|EndAbility))))
    (:OnCompleted
      (Ability|EndAbility :!label _label))
    (:OnInterrupted
      (goto _label))
    (:OnCancelled
      (goto _label))))