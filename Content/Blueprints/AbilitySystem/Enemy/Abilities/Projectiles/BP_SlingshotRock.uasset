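; BP_SlingshotRock is the rock projectile for an enemy slingshot ability, and this Blueprint gives it a randomized tumble.
; On BeginPlay it picks independent random roll, pitch and yaw rates, each either positive or negative.
; Tick scales those rates by delta time and adds them as local rotation to RockMesh, so the spin is frame-rate independent.
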(event EventBeginPlay
  (Utilities|FlowControl|Sequence
    (:then_0
      (Variables|Default|SetRollRotationRate (Math|Random|RandomFloatinRange -1e+02 1e+02)))
    (:then_1
      (Variables|Default|SetPitchRotationRate (Math|Random|RandomFloatinRange -1e+02 1e+02)))
    (:then_2
      (Variables|Default|SetYawRotationRate (Math|Random|RandomFloatinRange -1e+02 1e+02)))))

(event EventTick
  (params (DeltaSeconds :type Float%20%28single-precision%29))
  (Transformation|AddLocalRotation (Variables|Default|GetRockMesh) (Math|Rotator|MakeRotator (* DeltaSeconds (Variables|Default|GetRollRotationRate)) (* DeltaSeconds (Variables|Default|GetPitchRotationRate)) (* DeltaSeconds (Variables|Default|GetYawRotationRate))) false false))

(fn ConstructionScript)