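; Gameplay ability for the Fire Bolt spell, which casts a projectile at the point under the mouse.
; Target data supplies the impact point, which is passed through the avatar's CombatInterface to update its facing target for motion warping.
; It then plays the cast montage and waits for the Event.Montage.FireBolt gameplay event to time the projectile spawn.
; The ability ends after a short delay following the spawn.
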(event Ability|EventActivateAbility
  (bind _datahandle (|TargetDataUnderMouse)
    (:ValidData
      (Variables|Default|SetProjectileTargetLocation (.ImpactPoint (Collision|BreakHitResult (Ability|TargetData|GetHitResultfromTargetData _datahandle))))
      ;[1 1 1] 모션 워핑에서 이 부분을 좀 더 유연하게 하려면 전투 인터페이스에서 구현하고 이걸 전투 인터페이스에서 받아오도록 하면 전투하는 모든 캐릭터에 사용 가능
      (bind _ascombat_interface (Utilities|Casting|CastToCombatInterface (Ability|GetAvatarActorfromActorInfo)))
      (Class|CombatInterface|UpdateFacingTarget _ascombat_interface (Variables|Default|GetProjectileTargetLocation))
      (|PlayMontageandWaitProxy "None" "/Game/Assets/Characters/Aura/Animations/Abilities/AM_Cast_FireBolt.AM_Cast_FireBolt" 1.0 "None" true 1.0 0.0 false
        (:then
          (Ability|Tasks|WaitGameplayEvent "(TagName=\"Event.Montage.FireBolt\")" 0
            (:EventReceived
              (Class|AuraProjectileSpell|SpawnProjectile (Variables|Default|GetProjectileTargetLocation))
              (Utilities|FlowControl|Delay 0.5)
              (Ability|EndAbility))))))))

(event Ability|EventOnEndAbility
  (params (bWasCancelled :type Boolean)))